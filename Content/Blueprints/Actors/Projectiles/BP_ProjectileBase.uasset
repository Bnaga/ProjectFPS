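; Base projectile actor that delivers ammo damage when its projectile movement stops on impact.
; Depending on a flag, it either messages the hit actor with direct damage or sphere-overlaps pawns and dynamic objects within the ammo's damage radius, ignoring the player's current weapon.
; Radius hits also spawn an explosion impulse actor.
; Every impact hides the mesh, spawns an impact effect and expires the projectile shortly after.
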(event OnProjectileStop(ProjectileMovement)
  (params (ImpactResult :type Hit%20Result%20Structure%20%28by%20ref%29))
  (CallFunction|ProjectileStop ImpactResult))

(event EventBeginPlay
  (bind _asfps_character (Utilities|Casting|CastToFPS_Character (Game|Player|GetPlayerPawn 0)))
  (Variables|Default|SetPlayerRef _asfps_character))

(fn ConstructionScript)

(fn ProjectileStop
  (params (HitResult :type Hit%20Result%20Structure))
  (bind _mesh (Variables|Default|GetMesh))
  (Utilities|FlowControl|Sequence
    (:then_0
      (if (Variables|Default|GetIsCausingRadiusDamage)
        (CallFunction|ExplodeonImpact HitResult)
        (else
          (Class|TakeDamage|TakeDamage(Message) (.HitActor (Collision|BreakHitResult HitResult)) (Variables|Default|GetAmmoData) (Variables|Default|GetCriticalHitModifier) HitResult))))
    (:then_1
      (Development|SetHiddeninGame _mesh true false)
      (Game|SpawnActorfromClass (Variables|Default|GetImpactEffect) (Transformation|GetWorldTransform _mesh) "AlwaysSpawn" 0 HitResult true 0)
      (Actor|SetLifeSpan 0.1))))

(fn ExplodeonImpact
  (params (HitResult :type Hit%20Result%20Structure))
  (bind _impactpoint (Collision|BreakHitResult HitResult))
  (Utilities|FlowControl|Sequence
    (:then_0
      (bind _outactors (Collision|SphereOverlapActors _impactpoint (.DamageRadius (Utilities|Struct|BreakAmmoData (Variables|Default|GetAmmoData))) (Utilities|Array|MakeArray "ObjectTypeQuery2" "ObjectTypeQuery3") 0 (Utilities|Array|MakeArray (Variables|/Game/Blueprints/FPS_Character.FPS_Character_C|GetCurrentWeapon (Variables|Default|GetPlayerRef)))))
      (for _array_element _outactors
        (Class|TakeDamage|TakeRadiusDamage(Message) _array_element HitResult (Variables|Default|GetAmmoData) (Variables|Default|GetCriticalHitModifier))))
    (:then_1
      (Game|SpawnActorfromClass "/Game/Blueprints/Actors/Impulses/BP_ExplosionImpulse.BP_ExplosionImpulse_C" (Math|Transform|MakeTransform _impactpoint "0, 0, 0" "1,1,1") "AlwaysSpawn" 0 0))))