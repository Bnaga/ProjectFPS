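; FPS_PlayerController is a player controller that handles mouse look for the first-person character.
; On BeginPlay it casts the player pawn to FPS_Character and caches the reference.
; MouseX and MouseY feed yaw and pitch input, cut to a third while the character is aiming with one specific weapon type, giving finer aim.
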(event EventBeginPlay
  (bind _asfps_character (Utilities|Casting|CastToFPS_Character (Game|Player|GetPlayerPawn 0)))
  (Variables|Default|SetPlayerRef _asfps_character))

(event Input|AxisEvents|InputAxisMouseX
  (params (AxisValue :type Float%20%28single-precision%29))
  (bind _playerref (Variables|Default|GetPlayerRef))
  (Class|PlayerController|AddYawInput (select (and (Variables|/Game/Blueprints/FPS_Character.FPS_Character_C|GetIsAiming _playerref) (Utilities|Enum|Equal(Enum) (Variables|/Game/Blueprints/FPS_Character.FPS_Character_C|GetHasWeaponEnum _playerref) "NewEnumerator1")) (/ AxisValue 3.0) AxisValue)))

(event Input|AxisEvents|InputAxisMouseY
  (params (AxisValue :type Float%20%28single-precision%29))
  (bind _playerref (Variables|Default|GetPlayerRef))
  (Class|PlayerController|AddPitchInput (select (and (Variables|/Game/Blueprints/FPS_Character.FPS_Character_C|GetIsAiming _playerref) (Utilities|Enum|Equal(Enum) (Variables|/Game/Blueprints/FPS_Character.FPS_Character_C|GetHasWeaponEnum _playerref) "NewEnumerator1")) (/ AxisValue 3.0) AxisValue)))

(fn ConstructionScript)